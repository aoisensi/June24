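; Player camera pawn with an orthographic view that pans, zooms and places markers in the world.
; Tick consumes the pending movement input vector and applies it, scaled by delta time, as an unswept world offset.
; The ZoomCamera event adjusts the camera's ortho width from its input value.
; Left click traces under the cursor against WorldStatic objects and spawns a scaled-down BP_Marker at the hit location.
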(event Custom|ZoomCamera
  (params (Value :type Float%20%28single-precision%29))
  (bind _camera (Variables|Default|GetCamera))
  (Class|CameraComponent|SetOrthoWidth _camera (+ (Variables|/Script/Engine.CameraComponent|GetOrthoWidth _camera) (* Value -1e+02))))

(event EventTick
  (params (DeltaSeconds :type Float%20%28single-precision%29))
  ;[1 1 1] Camera Move
  (bind _returnvalue (Class|Pawn|ConsumeMovementInputVector))
  (Transformation|AddActorWorldOffset (* _returnvalue DeltaSeconds)))

(event Input|MouseEvents|LeftMouseButton
  (params (Key :type Key%20Structure :default "AnyKey"))
  (bind _returnvalue (Game|GetPlayerController 0))
  (bind _array (Utilities|Array|MakeArray "ObjectTypeQuery1"))
  (bind (_hitresult _returnvalue_2) (Class|PlayerController|GetHitResultUnderCursorforObjects _returnvalue _array true))
  (:Pressed
    (if _returnvalue_2
      (Game|SpawnActorfromClass "/Game/Base/Blueprints/BP_Marker.BP_Marker_C" (Math|Transform|MakeTransform (.Location (Collision|BreakHitResult _hitresult)) "0, 0, 0" "0.100000,0.100000,0.100000") "Undefined" 0 0))))

(fn ConstructionScript)