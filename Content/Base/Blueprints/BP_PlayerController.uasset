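; BP_PlayerController is a player controller that turns camera pan and zoom axis input into movement of the controlled pawn.
; Horizontal and vertical pan axes add movement input along fixed world Y and X directions, scaled by PanSpeed.
; The zoom axis casts the pawn to BP_PlayerCamera and passes the value to its ZoomCamera function.
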(event Input|ActionEvents|InputActionMove
  (params (Key :type Key%20Structure :default "AnyKey")))

(event Input|AxisEvents|InputAxisPanHorizon
  (params (AxisValue :type Float%20%28single-precision%29))
  (Pawn|Input|AddMovementInput (Game|Player|GetPlayerPawn 0) "0.000000,1.000000, 0" (* AxisValue (Variables|Default|GetPanSpeed)) false))

(event Input|AxisEvents|InputAxisPanVertical
  (params (AxisValue :type Float%20%28single-precision%29))
  (Pawn|Input|AddMovementInput (Game|Player|GetPlayerPawn 0) "1.000000, 0, 0" (* AxisValue (Variables|Default|GetPanSpeed)) false))

(event Input|AxisEvents|InputAxisCameraZoom
  (params (AxisValue :type Float%20%28single-precision%29))
  (bind _asbp_player_camera (Utilities|Casting|CastToBP_PlayerCamera (Game|Player|GetPlayerPawn 0)))
  (Default|ZoomCamera _asbp_player_camera AxisValue))

(fn ConstructionScript)