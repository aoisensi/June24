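; BP_Ant is an ant pawn that steers itself between overlapping BP_Marker actors by following the highest Dilution value.
; Every tick it scans the markers overlapping its capsule, keeps whichever beats its stored Marker and copies that Dilution onto itself.
; It then issues AIMoveTo toward the chosen marker, re-requested each tick while markers overlap, and lowers that marker's Dilution by one when a move succeeds.
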(event Custom|GoToMarker
  (bind _capsule (Variables|Default|GetCapsule))
  (bind _overlappingactors (Collision|GetOverlappingActors _capsule "/Game/Base/Blueprints/BP_Marker.BP_Marker_C" :!class /Script/Engine.PrimitiveComponent))
  (if (!= (Utilities|Array|Length _overlappingactors) 0)
    (for _array_element _overlappingactors
      (bind _asbp_marker (Utilities|Casting|CastToBP_Marker _array_element))
      (Utilities|IsValid (Variables|Default|GetMarker)
        (:Is%20Valid
          (if (< (Variables|/Game/Base/Blueprints/BP_Marker.BP_Marker_C|GetDilution (Variables|Default|GetMarker)) (Variables|/Game/Base/Blueprints/BP_Marker.BP_Marker_C|GetDilution _asbp_marker))
            (Variables|Default|SetMarker _asbp_marker)
            (Variables|Default|SetDilution (Variables|/Game/Base/Blueprints/BP_Marker.BP_Marker_C|GetDilution _asbp_marker))))
        (:Is%20Not%20Valid
          (Variables|Default|SetMarker _asbp_marker)
          (Variables|Default|SetDilution (Variables|/Game/Base/Blueprints/BP_Marker.BP_Marker_C|GetDilution _asbp_marker)))))
    (AI|AIMoveTo self "0, 0, 0" (Variables|Default|GetMarker) 5.0 false
      (:OnSuccess
        (Variables|/Game/Base/Blueprints/BP_Marker.BP_Marker_C|SetDilution (Variables|Default|GetMarker) (- (Variables|/Game/Base/Blueprints/BP_Marker.BP_Marker_C|GetDilution (Variables|Default|GetMarker)) 1))))))

(event EventTick
  (params (DeltaSeconds :type Float%20%28single-precision%29))
  (CallFunction|GotoMarker))

(fn ConstructionScript
  (|CallParentFunction))